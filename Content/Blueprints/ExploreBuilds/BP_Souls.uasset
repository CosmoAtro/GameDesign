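; BP_Souls is a will-o'-wisp pickup that floats in the level until the player character touches it.
; Two timelines alternate forward and reverse in an endless loop, driving the Willowisp component's relative location.
; Overlap on Coll casts to BP_ThirdPersonCharacterCustom, sets its WillowispCount to zero, prints debug text and destroys the actor.
; An increment of that count exists but is left unconnected.
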(event OnComponentBeginOverlap(Coll)
  (params (OverlappedComponent :type Primitive%20Component%20Object%20Reference) (OtherActor :type Actor%20Object%20Reference) (OtherComp :type Primitive%20Component%20Object%20Reference) (OtherBodyIndex :type Integer) (bFromSweep :type Boolean) (SweepResult :type Hit%20Result%20Structure%20%28by%20ref%29))
  (Development|PrintString "Hello")
  (bind _asbp_third_person_character_custom (Utilities|Casting|CastToBP_ThirdPersonCharacterCustom OtherActor))
  (Variables|/Game/Blueprints/allprevoiusstuff/BP_ThirdPersonCharacterCustom.BP_ThirdPersonCharacterCustom_C|Setwill-o'-wisp%20Count _asbp_third_person_character_custom 0)
  (Development|PrintString "will-o'-wisp count" true true "(R=0.103427,G=1.000000,B=0.634188,A=1.000000)")
  (Actor|DestroyActor))

(event EventBeginPlay
  (bind _newtrack_1 (Timeline|Timeline Play)
    (:Update
      (Transformation|SetRelativeLocation (Variables|Default|Getwill-o'-wisp) _newtrack_1 false false))
    (:Finished
      (bind _newtrack_1_2 (Timeline|Timeline_0 ReverseFromEnd)
        (:Update
          (Transformation|SetRelativeLocation (Variables|Default|Getwill-o'-wisp) _newtrack_1_2 false false))
        (:Finished
          (Timeline|Timeline PlayFromStart))))))

(event EventTick
  (params (DeltaSeconds :type Float%20%28single-precision%29)))

(fn ConstructionScript)